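; BP_Door_Small is a small sci-fi door actor that animates when something overlaps its Trigger component.
; Trigger overlap plays the skeletal door animation, swaps a wall material slot to green and activates the door-open sound cue.
; The IsOpen flag acts as a one-shot gate, cleared after firing.
; End overlap does nothing, and the reverse-playback closing logic is left disconnected.
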(event OnComponentBeginOverlap(Trigger)
  (params (OverlappedComponent :type Primitive%20Component%20Object%20Reference) (OtherActor :type Actor%20Object%20Reference) (OtherComp :type Primitive%20Component%20Object%20Reference) (OtherBodyIndex :type Integer) (bFromSweep :type Boolean) (SweepResult :type Hit%20Result%20Structure%20%28by%20ref%29))
  (if (Variables|Default|GetIsOpen)
    (Components|Animation|PlayAnimation (Variables|Default|GetSK_Door_Small) "/Game/Sci_Fi_Modular_Kit/Mesh/Skeletal_Meshes/SK_Door_Small_Anim.SK_Door_Small_Anim" false)
    (Rendering|Material|SetMaterial (Variables|Default|GetSM_Wall_Door_4x4) 8 "/Game/Sci_Fi_Modular_Kit/Materials/Decals/MI_UI_Green.MI_UI_Green")
    (Components|Activation|Activate (Variables|Default|GetSci_Fi_Door_Open_Cue) false)
    (Variables|Default|SetIsOpen false)))

(event OnComponentEndOverlap(Trigger)
  (params (OverlappedComponent :type Primitive%20Component%20Object%20Reference) (OtherActor :type Actor%20Object%20Reference) (OtherComp :type Primitive%20Component%20Object%20Reference) (OtherBodyIndex :type Integer)))

(event EventBeginPlay)

(event Collision|EventActorBeginOverlap
  (params (OtherActor :type Actor%20Object%20Reference)))

(event EventTick
  (params (DeltaSeconds :type Float%20%28single-precision%29)))

(fn ConstructionScript)