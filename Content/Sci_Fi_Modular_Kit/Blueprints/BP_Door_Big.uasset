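; BP_Door_Big is a large animated door that reacts to overlaps with its Trigger component.
; On begin overlap it plays the skeletal mesh's door animation, or takes the reverse path if DoorState is true; this file never sets that flag.
; End overlap always takes the reverse path, which sets a negative play rate and plays.
; Both paths act only while no animation is playing.
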(event OnComponentBeginOverlap(Trigger)
  (params (OverlappedComponent :type Primitive%20Component%20Object%20Reference) (OtherActor :type Actor%20Object%20Reference) (OtherComp :type Primitive%20Component%20Object%20Reference) (OtherBodyIndex :type Integer) (bFromSweep :type Boolean) (SweepResult :type Hit%20Result%20Structure%20%28by%20ref%29))
  (bind _sk_door_big_animated (Variables|Default|GetSK_Door_Big_Animated))
  (if (Variables|Default|GetDoor_State)
    (if (not (Audio|Components|Audio|IsPlaying _sk_door_big_animated))
      (Components|Timeline|SetPlayRate _sk_door_big_animated -1.0)
      (Audio|Components|Audio|Play _sk_door_big_animated false))
    (elif (not (Audio|Components|Audio|IsPlaying _sk_door_big_animated))
      (Components|Animation|PlayAnimation _sk_door_big_animated "/Game/Sci_Fi_Modular_Kit/Mesh/Skeletal_Meshes/SK_Door_Big_Animated_Anim.SK_Door_Big_Animated_Anim" false))))

(event OnComponentEndOverlap(Trigger)
  (params (OverlappedComponent :type Primitive%20Component%20Object%20Reference) (OtherActor :type Actor%20Object%20Reference) (OtherComp :type Primitive%20Component%20Object%20Reference) (OtherBodyIndex :type Integer))
  (bind _sk_door_big_animated (Variables|Default|GetSK_Door_Big_Animated))
  (if (not (Audio|Components|Audio|IsPlaying _sk_door_big_animated))
    (Components|Timeline|SetPlayRate _sk_door_big_animated -1.0)
    (Audio|Components|Audio|Play _sk_door_big_animated false)))

(event EventBeginPlay)

(event Collision|EventActorBeginOverlap
  (params (OtherActor :type Actor%20Object%20Reference)))

(event EventTick
  (params (DeltaSeconds :type Float%20%28single-precision%29)))

(fn ConstructionScript)