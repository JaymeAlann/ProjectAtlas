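; A large automatic sci-fi sliding door that opens when something enters its trigger and closes when it leaves.
; On overlap, after a short delay, it activates four steam effects and plays the seal timeline, with the door timeline following slightly later.
; The timelines lerp two seals and two door panels between closed and open positions.
; On exit the panels reverse immediately and the seals follow after a delay.
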(event OnComponentBeginOverlap(Trigger)
  (params (OverlappedComponent :type Primitive%20Component%20Object%20Reference) (OtherActor :type Actor%20Object%20Reference) (OtherComp :type Primitive%20Component%20Object%20Reference) (OtherBodyIndex :type Integer) (bFromSweep :type Boolean) (SweepResult :type Hit%20Result%20Structure%20%28by%20ref%29))
  (bind _doorclosed (Variables|Door|GetDoorClosed))
  (bind _sealclosed (Variables|Door|GetSealClosed))
  (Utilities|FlowControl|Delay 0.3)
  (Components|Activation|Activate (Variables|Default|GetSteamDoor) false)
  (Utilities|FlowControl|Sequence
    (:then_0
      ;[0 0.4972 1] Seal Opening
      (bind _sealopeningalpha (Timeline|SealTimeline Play)
        (:Update
          (Utilities|FlowControl|Sequence
            (:then_0
              (Transformation|SetRelativeLocation (Variables|Default|GetSM_DoorLarge_Seal) (Math|Vector|Lerp(Vector) _sealclosed (Variables|Door|GetSeal1Open) _sealopeningalpha) false false))
            (:then_1
              (Transformation|SetRelativeLocation (Variables|Default|GetSM_DoorLarge_Seal2) (Math|Vector|Lerp(Vector) _sealclosed (Variables|Door|GetSeal2Open) _sealopeningalpha) false false))))))
    (:then_1
      (Utilities|FlowControl|Delay 0.25)
      ;[0 0.4972 1] Door Opening
      (bind _doorposition (Timeline|DoorOpeningTimeline Play)
        (:Update
          (Utilities|FlowControl|Sequence
            (:then_0
              (Transformation|SetRelativeLocation (Variables|Default|GetSM_Door_Large_A_Right) (Math|Vector|Lerp(Vector) _doorclosed (Variables|Door|GetDoorOpenRight) _doorposition) false false))
            (:then_1
              (Transformation|SetRelativeLocation (Variables|Default|GetSM_Door_Large_A_Left) (Math|Vector|Lerp(Vector) _doorclosed (Variables|Door|GetDoorOpenLeft) _doorposition) false false))))))))

(event OnComponentEndOverlap(Trigger)
  (params (OverlappedComponent :type Primitive%20Component%20Object%20Reference) (OtherActor :type Actor%20Object%20Reference) (OtherComp :type Primitive%20Component%20Object%20Reference) (OtherBodyIndex :type Integer))
  (bind _doorclosed (Variables|Door|GetDoorClosed))
  (bind _sealclosed (Variables|Door|GetSealClosed))
  (Utilities|FlowControl|Sequence
    (:then_0
      (Utilities|FlowControl|Delay 1.25)
      ;[0 0.4972 1] Seal Opening
      (bind _sealopeningalpha (Timeline|SealTimeline Reverse)
        (:Update
          (Utilities|FlowControl|Sequence
            (:then_0
              (Transformation|SetRelativeLocation (Variables|Default|GetSM_DoorLarge_Seal) (Math|Vector|Lerp(Vector) _sealclosed (Variables|Door|GetSeal1Open) _sealopeningalpha) false false))
            (:then_1
              (Transformation|SetRelativeLocation (Variables|Default|GetSM_DoorLarge_Seal2) (Math|Vector|Lerp(Vector) _sealclosed (Variables|Door|GetSeal2Open) _sealopeningalpha) false false))))))
    (:then_1
      ;[0 0.4972 1] Door Opening
      (bind _doorposition (Timeline|DoorOpeningTimeline Reverse)
        (:Update
          (Utilities|FlowControl|Sequence
            (:then_0
              (Transformation|SetRelativeLocation (Variables|Default|GetSM_Door_Large_A_Right) (Math|Vector|Lerp(Vector) _doorclosed (Variables|Door|GetDoorOpenRight) _doorposition) false false))
            (:then_1
              (Transformation|SetRelativeLocation (Variables|Default|GetSM_Door_Large_A_Left) (Math|Vector|Lerp(Vector) _doorclosed (Variables|Door|GetDoorOpenLeft) _doorposition) false false))))))))

(fn ConstructionScript)