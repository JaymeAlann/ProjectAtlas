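; Free-flying spectator character, from the AlienPlants_Vol2 content, with a spotlight toggled by the T key.
; Movement inputs follow the camera's forward, right and up vectors.
; Mouse turn rotates controller yaw, while look-up pitches the spring arm only when no head-mounted display is enabled.
; Speed inputs scale a clamped Speed multiplicatively and write it to player 0's CharacterMovement max acceleration, not max speed.
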(event Input|ActionEvents|InputActionIncrease_Speed
  (params (Key :type Key%20Structure :default "AnyKey"))
  ;[1 1 1] Change Speed
  (:Pressed
    (bind _output_get (Variables|Default|SetSpeed (Math|Float|Clamp(Float) (* (Variables|Default|GetSpeed) 1.4) (Variables|Default|GetMinSpeed) (Variables|Default|GetMaxSpeed))))
    (Variables|/Script/Engine.CharacterMovementComponent|SetMaxAcceleration (Variables|/Script/Engine.Character|GetCharacterMovement (Game|GetPlayerCharacter 0)) _output_get)))

(event Input|ActionEvents|InputActionDecrease_Speed
  (params (Key :type Key%20Structure :default "AnyKey"))
  ;[1 1 1] Change Speed
  (:Pressed
    (bind _output_get (Variables|Default|SetSpeed (Math|Float|Clamp(Float) (/ (Variables|Default|GetSpeed) 1.4) (Variables|Default|GetMinSpeed) (Variables|Default|GetMaxSpeed))))
    (Variables|/Script/Engine.CharacterMovementComponent|SetMaxAcceleration (Variables|/Script/Engine.Character|GetCharacterMovement (Game|GetPlayerCharacter 0)) _output_get)))

(event Input|AxisEvents|InputAxisMoveUp
  (params (AxisValue :type Float%20%28single-precision%29))
  ;[1 1 1] Movement
  (Pawn|Input|AddMovementInput (Math|Vector|GetUpVector (Variables|/Script/Engine.PlayerCameraManager|GetTransformComponent (Game|GetPlayerCameraManager 0))) AxisValue true))

(event Input|AxisEvents|InputAxisMoveRight
  (params (AxisValue :type Float%20%28single-precision%29))
  ;[1 1 1] Movement
  (Pawn|Input|AddMovementInput (Math|Vector|GetRightVector (Variables|/Script/Engine.PlayerCameraManager|GetTransformComponent (Game|GetPlayerCameraManager 0))) AxisValue true))

(event Input|AxisEvents|InputAxisTurn
  (params (AxisValue :type Float%20%28single-precision%29))
  ;[1 1 1] Rotation
  (Pawn|Input|AddControllerYawInput (* (* AxisValue (Variables|Default|GetMouseSpeed)) 0.65)))

(event Input|AxisEvents|InputAxisLookUp
  (params (AxisValue :type Float%20%28single-precision%29))
  ;[1 1 1] Rotation
  (if (not (Class|HeadMountedDisplayFunctionLibrary|IsHeadMountedDisplayEnabled))
    (Transformation|AddRelativeRotation (Variables|Default|GetSpringArm) (Math|Rotator|MakeRotator 0.0 (* (* AxisValue (Variables|Default|GetMouseSpeed)) -1.0) 0.0) false false)))

(event Input|AxisEvents|InputAxisMoveForward
  (params (AxisValue :type Float%20%28single-precision%29))
  ;[1 1 1] Movement
  (Pawn|Input|AddMovementInput (Math|Vector|GetForwardVector (Variables|/Script/Engine.PlayerCameraManager|GetTransformComponent (Game|GetPlayerCameraManager 0))) AxisValue true))

(event Input|KeyboardEvents|T
  (params (Key :type Key%20Structure :default "AnyKey"))
  (:Pressed
    (Rendering|ToggleVisibility (Variables|Default|GetSpotLight) false)))

(fn ConstructionScript)