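; Glowing sphere actor for the AlienPlants_Vol2 pack whose point light dims as daylight rises.
; The construction script applies the configurable light radius and intensity to the light.
; The Update_Light event reads the AlienPlants_Daylight scalar from the MPC_APV2 parameter collection, inverts it to scale intensity, and hides the light when that inverted value is low.
; Nothing in this Blueprint calls Update_Light.
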(event Custom|Update_Light
  (bind _returnvalue (Rendering|Material|GetScalarParameterValue "/Game/AlienPlants_Vol2/Materials/MaterialFunctions/MPC_APV2.MPC_APV2" "AlienPlants_Daylight" :!class /Script/Engine.KismetMaterialLibrary))
  (Rendering|SetVisibility (Variables|Default|GetPointLight) (> (Math|Float|Lerp 1.0 0.0 _returnvalue) 0.2) false)
  (Rendering|Components|Light|SetIntensity (Variables|Default|GetPointLight) (* (Math|Float|Lerp 1.0 0.0 _returnvalue) (Variables|Default|GetLight_Intensity))))

(fn ConstructionScript
  (Rendering|Lighting|SetAttenuationRadius (Variables|Default|GetPointLight) (Variables|Default|GetLight_Radius))
  (Rendering|Components|Light|SetIntensity (Variables|Default|GetPointLight) (Variables|Default|GetLight_Intensity)))