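; Master Blueprint for sci-fi props that exposes emissive and color customization per actor.
; Its Construction Script gathers every static mesh component under the root, including nested children, into an array.
; It then pushes emissive power and color, three base colors, metallic color and a custom-color toggle to their materials as named parameters.
; The Event Graph holds no active logic.
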(event EventBeginPlay)

(event Collision|EventActorBeginOverlap
  (params (OtherActor :type Actor%20Object%20Reference)))

(event EventTick
  (params (DeltaSeconds :type Float%20%28single-precision%29)))

(fn ConstructionScript
  (bind _staticmeshcomponentstoedit (Variables|Default|GetStaticMeshComponentsToEdit))
  (Utilities|FlowControl|Sequence
    (:then_0
      (Utilities|Array|Clear (Variables|Default|GetStaticMeshComponentsToEdit))
      (for _array_element (Components|GetChildrenComponents (Variables|Default|GetRoot) true)
        (bind _asstatic_mesh_component (Utilities|Casting|CastToStaticMeshComponent _array_element))
        (Utilities|Array|Add (Variables|Default|GetStaticMeshComponentsToEdit) _asstatic_mesh_component)))
    (:then_1
      (Utilities|FlowControl|Sequence
        (:then_0
          (Rendering|Material|SetScalarParameterValueonMaterials _staticmeshcomponentstoedit "EmissivePower" (Variables|Emissive|GetEmissivePower)))
        (:then_1
          (Rendering|Material|SetVectorParameterValueonMaterials _staticmeshcomponentstoedit "EmissiveColor" (Math|Conversions|ToVector(LinearColor) (Variables|Emissive|GetEmissiveColor))))
        (:then_2
          (Rendering|Material|SetVectorParameterValueonMaterials _staticmeshcomponentstoedit "Color01" (Math|Conversions|ToVector(LinearColor) (Variables|CustomColor|GetColor01)))
          (Rendering|Material|SetVectorParameterValueonMaterials _staticmeshcomponentstoedit "Color02" (Math|Conversions|ToVector(LinearColor) (Variables|CustomColor|GetColor02)))
          (Rendering|Material|SetVectorParameterValueonMaterials _staticmeshcomponentstoedit "Color03" (Math|Conversions|ToVector(LinearColor) (Variables|CustomColor|GetColor03)))
          (Rendering|Material|SetVectorParameterValueonMaterials _staticmeshcomponentstoedit "MetallicColor" (Math|Conversions|ToVector(LinearColor) (Variables|CustomColor|GetMetallicColor))))
        (:then_3
          (Rendering|Material|SetScalarParameterValueonMaterials _staticmeshcomponentstoedit "isCustomColors" (Math|Conversions|ToFloat(Boolean) (Variables|CustomColor|GetisCustomColors))))))))