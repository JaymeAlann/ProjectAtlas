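; Interactive control panel prop with a hinged door, six fuses and an inside wire.
; BeginPlay hides any fuse or wire whose flag is off.
; On authority, ConnectActor routes the hit component to a timeline-driven door toggle or to showing flagged parts, with fuses grouped three per collision.
; The construction script chains one dynamic material through all meshes and sets its wear and roughness parameters.
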(event Custom|ShowWire
  (Rendering|SetVisibility (Variables|Default|GetSM_cp02WireInside) true false))

(event Custom|HideWire
  (Rendering|SetVisibility (Variables|Default|GetSM_cp02WireInside) false false))

(event Custom|CloseDoor
  (bind _doorangle (Timeline|OpenDoorTimeLine Reverse)
    (:Update
      (Transformation|SetRelativeRotation (Variables|Default|GetSM_cp2_02) (Math|Rotator|MakeRotator 0.0 0.0 _doorangle) false false))))

(event Custom|ShowFuse06
  (Rendering|SetVisibility (Variables|Default|GetSM_cp2Fuse_06) true false))

(event Custom|HideFuse06
  (Rendering|SetVisibility (Variables|Default|GetSM_cp2Fuse_06) false false))

(event Custom|ShowFuse01
  (Rendering|SetVisibility (Variables|Default|GetSM_cp2Fuse_01) true false))

(event Custom|HideFuse01
  (Rendering|SetVisibility (Variables|Default|GetSM_cp2Fuse_01) false false))

(event Custom|ShowFuse02
  (Rendering|SetVisibility (Variables|Default|GetSM_cp2Fuse_02) true false))

(event Custom|HideFuse02
  (Rendering|SetVisibility (Variables|Default|GetSM_cp2Fuse_02) false false))

(event Custom|OpenDoor
  (bind _doorangle (Timeline|OpenDoorTimeLine Play)
    (:Update
      (Transformation|SetRelativeRotation (Variables|Default|GetSM_cp2_02) (Math|Rotator|MakeRotator 0.0 0.0 _doorangle) false false))))

(event Custom|ShowFuse03
  (Rendering|SetVisibility (Variables|Default|GetSM_cp2Fuse_03) true false))

(event Custom|ShowFuse04
  (Rendering|SetVisibility (Variables|Default|GetSM_cp2Fuse_04) true false))

(event Custom|HideFuse03
  (Rendering|SetVisibility (Variables|Default|GetSM_cp2Fuse_03) false false))

(event Custom|HIdeFuse04
  (Rendering|SetVisibility (Variables|Default|GetSM_cp2Fuse_04) false false))

(event Custom|ShowFuse05
  (Rendering|SetVisibility (Variables|Default|GetSM_cp2Fuse_05) true false))

(event Custom|HideFuse05
  (Rendering|SetVisibility (Variables|Default|GetSM_cp2Fuse_05) false false))

(event EventConnectActor
  (params (HitComponent :type Actor%20Component%20Object%20Reference))
  (Variables|Default|SetHitComponent HitComponent)
  (Networking|SwitchHasAuthority
    (:Authority
      (if (== (Variables|Default|GetHitComponent) (Variables|Default|GetSM_cp2_02))
        (Utilities|FlowControl|FlipFlop
          (:A
            (CallFunction|OpenDoor))
          (:B
            (CallFunction|CloseDoor)))
        (elif (== (Variables|Default|GetHitComponent) (Variables|Default|GetFuse1Collision))
          (if (Variables|Default|GetFuse1)
            (CallFunction|ShowFuse01))
          (if (Variables|Default|GetFuse2)
            (CallFunction|ShowFuse02))
          (if (Variables|Default|GetFuse3)
            (CallFunction|ShowFuse03))
          (elif (== (Variables|Default|GetHitComponent) (Variables|Default|GetFuse2Collision))
            (if (Variables|Default|GetFuse4)
              (CallFunction|ShowFuse04))
            (if (Variables|Default|GetFuse5)
              (CallFunction|ShowFuse05))
            (if (Variables|Default|GetFuse6)
              (CallFunction|ShowFuse06))
            (elif (== (Variables|Default|GetHitComponent) (Variables|Default|GetWireCollision))
              (if (Variables|Default|GetWire)
                (CallFunction|ShowWire)))))))))

(event EventBeginPlay
  (Utilities|FlowControl|Sequence
    (:then_0
      (if (not (Variables|Default|GetFuse1))
        (CallFunction|HideFuse01)))
    (:then_1
      (if (not (Variables|Default|GetFuse2))
        (CallFunction|HideFuse02)))
    (:then_2
      (if (not (Variables|Default|GetFuse3))
        (CallFunction|HideFuse03)))
    (:then_3
      (if (not (Variables|Default|GetFuse4))
        (CallFunction|HIdeFuse04)))
    (:then_4
      (if (not (Variables|Default|GetFuse5))
        (CallFunction|HideFuse05)))
    (:then_5
      (if (not (Variables|Default|GetFuse6))
        (CallFunction|HideFuse06)))
    (:then_6
      (if (not (Variables|Default|GetWire))
        (CallFunction|HideWire)))))

(fn ConstructionScript
  (bind _returnvalue (Rendering|Material|CreateDynamicMaterialInstance (Variables|Default|GetSM_cp2_01) 0 (Variables|Default|Getcp%20DM) :!class /Script/Engine.PrimitiveComponent))
  (bind _returnvalue_2 (Rendering|Material|CreateDynamicMaterialInstance (Variables|Default|GetSM_cp2Fuse_01) 0 _returnvalue :!class /Script/Engine.PrimitiveComponent))
  (bind _returnvalue_3 (Rendering|Material|CreateDynamicMaterialInstance (Variables|Default|GetSM_cp2Fuse_02) 0 _returnvalue_2 :!class /Script/Engine.PrimitiveComponent))
  (bind _returnvalue_4 (Rendering|Material|CreateDynamicMaterialInstance (Variables|Default|GetSM_cp2Fuse_03) 0 _returnvalue_3 :!class /Script/Engine.PrimitiveComponent))
  (bind _returnvalue_5 (Rendering|Material|CreateDynamicMaterialInstance (Variables|Default|GetSM_cp2Fuse_04) 0 _returnvalue_4 :!class /Script/Engine.PrimitiveComponent))
  (bind _returnvalue_6 (Rendering|Material|CreateDynamicMaterialInstance (Variables|Default|GetSM_cp2Fuse_05) 0 _returnvalue_5 :!class /Script/Engine.PrimitiveComponent))
  (bind _returnvalue_7 (Rendering|Material|CreateDynamicMaterialInstance (Variables|Default|GetSM_cp2Fuse_06) 0 _returnvalue_6 :!class /Script/Engine.PrimitiveComponent))
  (bind _returnvalue_8 (Rendering|Material|CreateDynamicMaterialInstance (Variables|Default|GetSM_cp2_02) 0 _returnvalue_7 :!class /Script/Engine.PrimitiveComponent))
  (bind _returnvalue_9 (Rendering|Material|CreateDynamicMaterialInstance (Variables|Default|GetSM_cp02WireInside) 0 _returnvalue_8 :!class /Script/Engine.PrimitiveComponent))
  (bind _output_get (Variables|Default|Setcp%20DM _returnvalue_9))
  (Rendering|Material|SetScalarParameterValue _output_get "a:old1" (Variables|Default|GetOld1) :!class /Script/Engine.MaterialInstanceDynamic)
  (Rendering|Material|SetScalarParameterValue (Variables|Default|Getcp%20DM) "b:old2" (Variables|Default|GetOld2) :!class /Script/Engine.MaterialInstanceDynamic)
  (Rendering|Material|SetScalarParameterValue (Variables|Default|Getcp%20DM) "c:full" (Variables|Default|GetFull) :!class /Script/Engine.MaterialInstanceDynamic)
  (Rendering|Material|SetScalarParameterValue (Variables|Default|Getcp%20DM) "d:mainroughness" (Variables|Default|GetMainRoughness) :!class /Script/Engine.MaterialInstanceDynamic))