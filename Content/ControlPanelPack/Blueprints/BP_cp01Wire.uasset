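; BP_cp01Wire is a modular wire prop for the control panel pack, built entirely in its Construction Script.
; In edit mode it stretches the middle mesh along local Z, moves and rotates the end piece, applies the chosen meshes, and optionally adds holder meshes at automatic intervals or listed offsets.
; Otherwise it snaps to a BP_cp01's "wire" socket or another wire's "endsocket", allowing chained segments.
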(event EventBeginPlay)

(event EventActorBeginOverlap
  (params (OtherActor :type Actor%20Object%20Reference)))

(event EventTick
  (params (DeltaSeconds :type Float%20%28single-precision%29)))

(fn ConstructionScript
  (bind _attachto (Variables|Default|GetAttachTo))
  (bind _length (Variables|Default|Getlength))
  (bind _holder (Variables|Default|Getholder))
  (bind _holderangle (Variables|Default|GetHolderAngle))
  (bind _holderlocation (Variables|Default|GetHolderLocation))
  (bind _holderscale (Variables|Default|GetHolderScale))
  (bind _holderlocation_2 (Variables|Default|GetHolderLocation))
  (bind _returnvalue (Utilities|Array|Length _holder))
  (bind _z (Math|Vector|BreakVector _length))
  (bind (_x _y _z_2) (Math|Vector|BreakVector _holderscale))
  (bind (_x_2 _y_2 _z_3) (Math|Vector|BreakVector _holderangle))
  (bind (_x_3 _y_3) (Math|Vector|BreakVector _holderlocation))
  (bind (_x_4 _y_4) (Math|Vector|BreakVector _holderlocation_2))
  (bind _returnvalue_2 (Math|Rotator|MakeRotator _x_2 _y_2 _z_3))
  (bind _returnvalue_3 (Math|Vector|MakeVector _x _y _z_2))
  (if (Variables|Default|GetEditMode?)
    ;[1 1 1] edit mode
    (Transformation|SetRelativeScale3D (Variables|Default|Getmiddle) (Math|Vector|MakeVector 1.0 1.0 (/ (* _z -1.0) 77.88)))
    (Transformation|SetRelativeLocation (Variables|Default|Getend) (Math|Vector|MakeVector 0.0 0.0 _z) false false)
    (Transformation|SetRelativeRotation (Variables|Default|Getend) (Math|Rotator|MakeRotator 0.0 0.0 (Math|Conversions|ToFloat(Integer) (Variables|Default|GetEndmeshAngle))) false false)
    (if (Variables|Default|GetHolder?)
      (if (Variables|Default|Getauto?)
        (bind _index (Utilities|FlowControl|ForLoopwithBreak 0 (Math|Float|Truncate (/ (* (.Z (Math|Vector|BreakVector (Variables|Default|Getlength))) -1.0) (Math|Conversions|ToFloat(Integer) (Variables|Default|Getautounit)))))
          (:LoopBody
            (if (<= (Math|Float|Truncate _z) (* (* (Variables|Default|Getautounit) -1) (+ _index 1)))
              (bind _returnvalue_4 (AddComponent|AddStaticMeshComponent false (Math|Transform|MakeTransform (Math|Vector|MakeVector 0.0 0.0 (* (Math|Conversions|ToFloat(Integer) (* (Variables|Default|Getautounit) (+ _index 1))) -1.0)) "0, 0,0.000000")))
              (Transformation|SetRelativeTransform _returnvalue_4 (Math|Transform|MakeTransform (Math|Vector|MakeVector _x_4 _y_4 (* (Math|Conversions|ToFloat(Integer) (* (Variables|Default|Getautounit) (+ _index 1))) -1.0)) _returnvalue_2 _returnvalue_3) false false))))
        (else
          (bind _index_2 (Utilities|FlowControl|ForLoopwithBreak 0 _returnvalue)
            (:LoopBody
              (if (!= _index_2 _returnvalue)
                (bind _returnvalue_5 (AddComponent|AddStaticMeshComponent false (Math|Transform|MakeTransform (Math|Vector|MakeVector 0.0 0.0 (Utilities|Array|Get(acopy) _holder _index_2)) "0, 0,0.000000")))
                (Transformation|SetRelativeTransform _returnvalue_5 (Math|Transform|MakeTransform (Math|Vector|MakeVector _x_3 _y_3 (Utilities|Array|Get(acopy) _holder _index_2)) _returnvalue_2 _returnvalue_3) false false)))))))
    (Components|StaticMesh|SetStaticMesh (Variables|Default|Getstart) (Variables|Default|Getstartmesh))
    (Components|StaticMesh|SetStaticMesh (Variables|Default|Getmiddle) (Variables|Default|Getmiddlemesh))
    (Components|StaticMesh|SetStaticMesh (Variables|Default|Getend) (Variables|Default|Getendmesh))
    (else
      ;[1 1 1] attach mode
      (Utilities|IsValid _attachto
        (:Is%20Valid
          (Utilities|FlowControl|Sequence
            (:then_0
              (bind _asbp_cp_01 (Utilities|Casting|CastToBP_cp01 _attachto))
              (Class|Actor|AttachRootComponenttoActor _asbp_cp_01 "wire" "SnapToTarget" true))
            (:then_1
              (bind _asbp_cp_01wire (Utilities|Casting|CastToBP_cp01Wire _attachto))
              (Class|Actor|AttachRootComponentto (Variables|BP_cp01Wire_C|Getend _asbp_cp_01wire) "endsocket" "SnapToTargetIncludingScale" true))))))))