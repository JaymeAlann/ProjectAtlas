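; Interactive control panel prop with a hinged timeline-driven door, a main switch, two sub switches and an inner wire.
; ConnectActor routes the passed hit component through FlipFlops to toggle the door and switches; the Wire flag controls whether the inner wire starts hidden or can be shown.
; Each switch or wire change calls Switch, which derives indicator lights from their states.
; A dynamic material created in the construction script carries wear and light parameters.
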(event Custom|Closedoor
  (bind _angle (Timeline|Open Reverse)
    (:Update
      (Transformation|SetRelativeRotation (Variables|Default|GetSM_cp05_02) (Math|Rotator|MakeRotator 0.0 0.0 _angle) false false))))

(event Custom|Switch
  (if (Rendering|IsVisible (Variables|Default|GetSM_cp05WireInside))
    (if (Variables|Default|GetMainSwitchOn?)
      (if (and (Variables|Default|GetSubSwitch01On?) (Variables|Default|GetSubSwitch02On?))
        (Rendering|Material|SetScalarParameterValue (Variables|Default|GetDM) "e:alert" 1.0 :!class /Script/Engine.MaterialInstanceDynamic)
        (Rendering|Material|SetScalarParameterValue (Variables|Default|GetDM) "f:power" 1.0 :!class /Script/Engine.MaterialInstanceDynamic)
        (Rendering|Material|SetScalarParameterValue (Variables|Default|GetDM) "g:stop" 1.0 :!class /Script/Engine.MaterialInstanceDynamic)
        (Rendering|Material|SetScalarParameterValue (Variables|Default|GetDM) "j:all" 1.0 :!class /Script/Engine.MaterialInstanceDynamic)
        (else
          (Rendering|Material|SetScalarParameterValue (Variables|Default|GetDM) "e:alert" 1.0 :!class /Script/Engine.MaterialInstanceDynamic)
          (Rendering|Material|SetScalarParameterValue (Variables|Default|GetDM) "f:power" 1.0 :!class /Script/Engine.MaterialInstanceDynamic)
          (Rendering|Material|SetScalarParameterValue (Variables|Default|GetDM) "g:stop" 1.0 :!class /Script/Engine.MaterialInstanceDynamic)
          (Rendering|Material|SetScalarParameterValue (Variables|Default|GetDM) "j:all" 0.0 :!class /Script/Engine.MaterialInstanceDynamic)))
      (else
        (Rendering|Material|SetScalarParameterValue (Variables|Default|GetDM) "e:alert" 1.0 :!class /Script/Engine.MaterialInstanceDynamic)
        (Rendering|Material|SetScalarParameterValue (Variables|Default|GetDM) "f:power" 0.0 :!class /Script/Engine.MaterialInstanceDynamic)
        (Rendering|Material|SetScalarParameterValue (Variables|Default|GetDM) "g:stop" 1.0 :!class /Script/Engine.MaterialInstanceDynamic)
        (Rendering|Material|SetScalarParameterValue (Variables|Default|GetDM) "j:all" 0.0 :!class /Script/Engine.MaterialInstanceDynamic)))
    (else
      (Rendering|Material|SetScalarParameterValue (Variables|Default|GetDM) "e:alert" 0.0 :!class /Script/Engine.MaterialInstanceDynamic)
      (Rendering|Material|SetScalarParameterValue (Variables|Default|GetDM) "f:power" 0.0 :!class /Script/Engine.MaterialInstanceDynamic)
      (Rendering|Material|SetScalarParameterValue (Variables|Default|GetDM) "g:stop" 0.0 :!class /Script/Engine.MaterialInstanceDynamic)
      (Rendering|Material|SetScalarParameterValue (Variables|Default|GetDM) "j:all" 0.0 :!class /Script/Engine.MaterialInstanceDynamic))))

(event Custom|MainSwitchOn
  (Transformation|SetRelativeRotation (Variables|Default|GetSM_cp05Switch_01) "-90.000000, 0, 0" false false)
  (Variables|Default|SetMainSwitchOn? true)
  (CallFunction|Switch))

(event Custom|MainSwitchOff
  (Transformation|SetRelativeRotation (Variables|Default|GetSM_cp05Switch_01) "0.000000, 0, 0" false false)
  (Variables|Default|SetMainSwitchOn? false)
  (CallFunction|Switch))

(event Custom|OpenDoor
  (bind _angle (Timeline|Open Play)
    (:Update
      (Transformation|SetRelativeRotation (Variables|Default|GetSM_cp05_02) (Math|Rotator|MakeRotator 0.0 0.0 _angle) false false))))

(event Custom|SubSwitch01On
  (Transformation|SetRelativeRotation (Variables|Default|GetSM_cp05Switch_02) "40.000000, 0, 0" false false)
  (Variables|Default|SetSubSwitch01On? true)
  (CallFunction|Switch))

(event Custom|SubSwitch01Off
  (Transformation|SetRelativeRotation (Variables|Default|GetSM_cp05Switch_02) "0.000000, 0, 0" false false)
  (Variables|Default|SetSubSwitch01On? false)
  (CallFunction|Switch))

(event Custom|SubSwitch02Off
  (Transformation|SetRelativeRotation (Variables|Default|GetSM_cp05Switch_03) "0.000000, 0, 0" false false)
  (Variables|Default|SetSubSwitch02On? false)
  (CallFunction|Switch))

(event Custom|ShowWire
  (Rendering|SetVisibility (Variables|Default|GetSM_cp05WireInside) true false)
  (CallFunction|Switch))

(event Custom|HideWire
  (Rendering|SetVisibility (Variables|Default|GetSM_cp05WireInside) false false)
  (CallFunction|Switch))

(event Custom|SubSwitch02On
  (Transformation|SetRelativeRotation (Variables|Default|GetSM_cp05Switch_03) "40.000000, 0, 0" false false)
  (Variables|Default|SetSubSwitch02On? true)
  (CallFunction|Switch))

(event EventBeginPlay
  (if (Variables|Default|GetWire?)
    (CallFunction|Switch)
    (else
      (CallFunction|HideWire)
      (CallFunction|Switch))))

(event EventConnectActor
  (params (HitComponent :type Actor%20Component%20Object%20Reference))
  (bind _output_get (Variables|Default|SetHitComponent HitComponent))
  (if (== _output_get (Variables|Default|GetSM_cp05_02))
    (Utilities|FlowControl|FlipFlop
      (:A
        (CallFunction|OpenDoor))
      (:B
        (CallFunction|Closedoor)))
    (elif (== (Variables|Default|GetHitComponent) (Variables|Default|GetSwitch01Collision))
      (Utilities|FlowControl|FlipFlop
        (:A
          (CallFunction|SubSwitch01on))
        (:B
          (CallFunction|SubSwitch01Off)))
      (elif (== (Variables|Default|GetHitComponent) (Variables|Default|GetSwitch02Collision))
        (Utilities|FlowControl|FlipFlop
          (:A
            (CallFunction|SubSwitch02on))
          (:B
            (CallFunction|SubSwitch02Off)))
        (elif (== (Variables|Default|GetHitComponent) (Variables|Default|GetSM_cp05Switch_01))
          (Utilities|FlowControl|FlipFlop
            (:A
              (CallFunction|MainSwitchon))
            (:B
              (CallFunction|MainSwitchOff)))
          (elif (== (Variables|Default|GetHitComponent) (Variables|Default|GetWireCollision))
            (if (Variables|Default|GetWire?)
              (CallFunction|ShowWire))))))))

(fn ConstructionScript
  (bind _returnvalue (Rendering|Material|CreateDynamicMaterialInstance "/Game/ControlPanelPack/Materials/M_cp05.M_cp05" :!class /Script/Engine.KismetMaterialLibrary))
  (bind _output_get (Variables|Default|SetDM _returnvalue))
  (Rendering|Material|SetMaterial (Variables|Default|GetSM_cp05_01) 0 _output_get)
  (Rendering|Material|SetScalarParameterValue (Variables|Default|GetDM) "a:old1" (Variables|Default|GetOld1) :!class /Script/Engine.MaterialInstanceDynamic)
  (Rendering|Material|SetScalarParameterValue (Variables|Default|GetDM) "b:old2" (Variables|Default|GetOld2) :!class /Script/Engine.MaterialInstanceDynamic)
  (Rendering|Material|SetScalarParameterValue (Variables|Default|GetDM) "c:full" (Variables|Default|GetFull) :!class /Script/Engine.MaterialInstanceDynamic)
  (Rendering|Material|SetScalarParameterValue (Variables|Default|GetDM) "d:mainroughness" (Variables|Default|GetMainRoughness) :!class /Script/Engine.MaterialInstanceDynamic)
  (Rendering|Material|SetScalarParameterValue (Variables|Default|GetDM) "e:alert" (Variables|Default|GetAlert) :!class /Script/Engine.MaterialInstanceDynamic)
  (Rendering|Material|SetScalarParameterValue (Variables|Default|GetDM) "f:power" (Variables|Default|GetPower) :!class /Script/Engine.MaterialInstanceDynamic)
  (Rendering|Material|SetScalarParameterValue (Variables|Default|GetDM) "g:stop" (Variables|Default|GetStop) :!class /Script/Engine.MaterialInstanceDynamic)
  (Rendering|Material|SetScalarParameterValue (Variables|Default|GetDM) "h:lightintensity" (Variables|Default|GetLightIntensity) :!class /Script/Engine.MaterialInstanceDynamic)
  (Rendering|Material|SetScalarParameterValue (Variables|Default|GetDM) "j:all" (Variables|Default|GetAllLight) :!class /Script/Engine.MaterialInstanceDynamic))