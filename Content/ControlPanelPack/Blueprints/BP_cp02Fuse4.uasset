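; Fuse pickup actor for the cp02 control panel in the Control Panel Pack, representing fuse number four.
; On ConnectActor it casts its ControlBox1 reference to BP_cp02, sets that panel's Fuse4 flag and destroys itself.
; The construction script creates a dynamic material instance on the fuse mesh and feeds it wear and roughness parameters from the actor's variables.
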(event EventConnectActor
  (params (HitComponent :type Actor%20Component%20Object%20Reference))
  (bind _controlbox1 (Variables|Default|GetControlBox1))
  (Utilities|IsValid _controlbox1
    (:Is%20Valid
      (bind _asbp_cp_02 (Utilities|Casting|CastToBP_cp02 _controlbox1))
      (Variables|/Game/ControlPanelPack/Blueprints/BP_cp02.BP_cp02_C|Setfuse4 _asbp_cp_02 true)
      (Actor|DestroyActor))))

(fn ConstructionScript
  (bind _returnvalue (Rendering|Material|CreateDynamicMaterialInstance (Variables|Default|GetSM_cp02Fuse_04) 0 (Variables|Default|Getcp%20DM) :!class /Script/Engine.PrimitiveComponent))
  (bind _output_get (Variables|Default|Setcp%20DM _returnvalue))
  (Rendering|Material|SetScalarParameterValue _output_get "a:old1" (Variables|Default|GetOld1) :!class /Script/Engine.MaterialInstanceDynamic)
  (Rendering|Material|SetScalarParameterValue (Variables|Default|Getcp%20DM) "b:old2" (Variables|Default|GetOld2) :!class /Script/Engine.MaterialInstanceDynamic)
  (Rendering|Material|SetScalarParameterValue (Variables|Default|Getcp%20DM) "c:full" (Variables|Default|GetFull) :!class /Script/Engine.MaterialInstanceDynamic)
  (Rendering|Material|SetScalarParameterValue (Variables|Default|Getcp%20DM) "d:mainroughness" (Variables|Default|GetMainRoughness) :!class /Script/Engine.MaterialInstanceDynamic))