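; Interactive control panel with a hinged door, lock, two fuse switches, push buttons and an attachable wire.
; ConnectActor routes the hit component on authority to events that animate parts and set state flags.
; Switch drives run, open or close material indicators, lit only when the wire is visible and both fuses are on.
; The construction script chains one dynamic material through the meshes and applies wear, roughness and light settings.
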(event Custom|PressStartButton
  (Transformation|SetRelativeLocation (Variables|Default|GetSM_cp01Button_02) "18.094604,4.971998,-27.074903" false false)
  (Transformation|SetRelativeLocation (Variables|Default|GetSM_cp01Button_03) "32.160759,6.971998,-27.074903" false false)
  (Transformation|SetRelativeLocation (Variables|Default|GetSM_cp01Button_04) "46.227417,6.971998,-27.074903" false false)
  (Variables|Default|SetRun? true)
  (CallFunction|Switch))

(event Custom|Switch
  (if (Math|Boolean|ANDBoolean (Rendering|IsVisible (Variables|Default|GetSM_cp01WireInside)) (Variables|Default|GetSwitch01On?) (Variables|Default|GetSwitch02On?))
    (if (Variables|Default|GetRun?)
      (Rendering|Material|SetScalarParameterValue (Variables|Default|Getcp%20DM) "b:run" 1.0 :!class /Script/Engine.MaterialInstanceDynamic)
      (Rendering|Material|SetScalarParameterValue (Variables|Default|Getcp%20DM) "c:open" 0.0 :!class /Script/Engine.MaterialInstanceDynamic)
      (Rendering|Material|SetScalarParameterValue (Variables|Default|Getcp%20DM) "d:close" 0.0 :!class /Script/Engine.MaterialInstanceDynamic)
      (elif (Variables|Default|GetOpen?)
        (Rendering|Material|SetScalarParameterValue (Variables|Default|Getcp%20DM) "b:run" 0.0 :!class /Script/Engine.MaterialInstanceDynamic)
        (Rendering|Material|SetScalarParameterValue (Variables|Default|Getcp%20DM) "c:open" 1.0 :!class /Script/Engine.MaterialInstanceDynamic)
        (Rendering|Material|SetScalarParameterValue (Variables|Default|Getcp%20DM) "d:close" 0.0 :!class /Script/Engine.MaterialInstanceDynamic)
        (else
          (Rendering|Material|SetScalarParameterValue (Variables|Default|Getcp%20DM) "b:run" 0.0 :!class /Script/Engine.MaterialInstanceDynamic)
          (Rendering|Material|SetScalarParameterValue (Variables|Default|Getcp%20DM) "c:open" 0.0 :!class /Script/Engine.MaterialInstanceDynamic)
          (Rendering|Material|SetScalarParameterValue (Variables|Default|Getcp%20DM) "d:close" 1.0 :!class /Script/Engine.MaterialInstanceDynamic))))
    (else
      (Rendering|Material|SetScalarParameterValue (Variables|Default|Getcp%20DM) "b:run" 0.0 :!class /Script/Engine.MaterialInstanceDynamic)
      (Rendering|Material|SetScalarParameterValue (Variables|Default|Getcp%20DM) "c:open" 0.0 :!class /Script/Engine.MaterialInstanceDynamic)
      (Rendering|Material|SetScalarParameterValue (Variables|Default|Getcp%20DM) "d:close" 0.0 :!class /Script/Engine.MaterialInstanceDynamic))))

(event Custom|TurnOnFuse01
  (Transformation|SetRelativeRotation (Variables|Default|GetSM_cp01Switch_01) "0, 0,-60.000000" false false)
  (Variables|Default|SetSwitch01On? true)
  (CallFunction|Switch))

(event Custom|TurnOffFuse01
  (Transformation|SetRelativeRotation (Variables|Default|GetSM_cp01Switch_01) "0, 0,60.000000" false false)
  (Variables|Default|SetSwitch01On? false)
  (CallFunction|Switch))

(event Custom|TurnOnFuse02
  (Transformation|SetRelativeRotation (Variables|Default|GetSM_cp01Switch_02) "0, 0,-60.000000" false false)
  (Variables|Default|SetSwitch02On? true)
  (CallFunction|Switch))

(event Custom|TurnOffFuse02
  (Transformation|SetRelativeRotation (Variables|Default|GetSM_cp01Switch_02) "0, 0,60.000000" false false)
  (Variables|Default|SetSwitch02On? false)
  (CallFunction|Switch))

(event Custom|PressMainSwitch
  (Transformation|SetRelativeLocation (Variables|Default|GetSM_cp01Button_01) "22.940559,5.410187,-1.322884" false false)
  (Variables|Default|SetRun? false)
  (CallFunction|Switch))

(event Custom|ReleaseMainSwitch
  (Transformation|SetRelativeLocation (Variables|Default|GetSM_cp01Button_01) "22.940559,8.700000,-1.322884" false false)
  (CallFunction|Switch))

(event Custom|RotateLock
  (Variables|Default|SetOpen? true)
  (bind _rotationvalue (Timeline|RotateLockTimeLine Play)
    (:Update
      (Transformation|SetRelativeRotation (Variables|Default|GetSM_cp01Lock_01) (Math|Rotator|MakeRotator 0.0 _rotationvalue 0.0) false false))
    (:Finished
      (CallFunction|Switch))))

(event Custom|ReverseLock
  (Variables|Default|SetOpen? false)
  (bind _rotationvalue (Timeline|RotateLockTimeLine Reverse)
    (:Update
      (Transformation|SetRelativeRotation (Variables|Default|GetSM_cp01Lock_01) (Math|Rotator|MakeRotator 0.0 _rotationvalue 0.0) false false))
    (:Finished
      (CallFunction|Switch))))

(event Custom|ReleaseStartButton
  (Transformation|SetRelativeLocation (Variables|Default|GetSM_cp01Button_02) "18.094604,6.971998,-27.074903" false false)
  (CallFunction|Switch))

(event Custom|AttachWire
  (Rendering|SetVisibility (Variables|Default|GetSM_cp01WireInside) true false)
  (CallFunction|Switch))

(event Custom|DetachWire
  (Rendering|SetVisibility (Variables|Default|GetSM_cp01WireInside) false false)
  (CallFunction|Switch))

(event Custom|PressResetButton
  (Transformation|SetRelativeLocation (Variables|Default|GetSM_cp01Button_03) "32.160767,4.971998,-27.074903" false false)
  (Transformation|SetRelativeLocation (Variables|Default|GetSM_cp01Button_02) "18.094604,6.971998,-27.074903" false false)
  (Transformation|SetRelativeLocation (Variables|Default|GetSM_cp01Button_04) "46.227417,6.971998,-27.074903" false false)
  (Transformation|SetRelativeLocation (Variables|Default|GetSM_cp01Button_01) "22.940559,8.700000,-1.322884" false false)
  (Variables|Default|SetRun? false)
  (CallFunction|Switch))

(event Custom|ReleaseResetButton
  (Transformation|SetRelativeLocation (Variables|Default|GetSM_cp01Button_03) "32.160759,6.971998,-27.074903" false false)
  (CallFunction|Switch))

(event Custom|OpenDoor
  (Components|Animation|PlayAnimation (Variables|Default|GetSK_cp01MWire) "/Game/ControlPanelPack/Animations/Anim_cp01MWireOpen.Anim_cp01MWireOpen" false)
  (Components|Animation|SetPosition (Variables|Default|GetSK_cp01MWire) 2.0 true)
  (bind _rotationvalue (Timeline|OpenDoorTimeLine Play)
    (:Update
      (Transformation|SetRelativeRotation (Variables|Default|GetSM_cp01_02) (Math|Rotator|MakeRotator 0.0 0.0 _rotationvalue) false false))))

(event Custom|PressStopButton
  (Transformation|SetRelativeLocation (Variables|Default|GetSM_cp01Button_04) "46.227417,4.971998,-27.074903" false false)
  (Transformation|SetRelativeLocation (Variables|Default|GetSM_cp01Button_03) "32.160759,6.971998,-27.074903" false false)
  (Transformation|SetRelativeLocation (Variables|Default|GetSM_cp01Button_02) "18.094604,6.971998,-27.074903" false false)
  (Variables|Default|SetRun? false)
  (CallFunction|Switch))

(event Custom|ReleaseStopButton
  (Transformation|SetRelativeLocation (Variables|Default|GetSM_cp01Button_04) "46.227417,6.971998,-27.074903" false false)
  (CallFunction|Switch))

(event Custom|CloseDoor
  (Components|Animation|PlayAnimation (Variables|Default|GetSK_cp01MWire) "/Game/ControlPanelPack/Animations/Anim_cp01MWireClose.Anim_cp01MWireClose" false)
  (Components|Timeline|SetPlayRate (Variables|Default|GetSK_cp01MWire) 2.0)
  (bind _rotationvalue (Timeline|OpenDoorTimeLine Reverse)
    (:Update
      (Transformation|SetRelativeRotation (Variables|Default|GetSM_cp01_02) (Math|Rotator|MakeRotator 0.0 0.0 _rotationvalue) false false))))

(event EventBeginPlay
  (CallFunction|CloseDoor)
  (CallFunction|Switch)
  (if (Variables|Default|GetWire1)
    (CallFunction|Switch)
    (else
      (CallFunction|DetachWire)
      (CallFunction|Switch))))

(event EventConnectActor
  (params (HitComponent :type Actor%20Component%20Object%20Reference))
  (Variables|Default|SetHitComponent HitComponent)
  (Networking|SwitchHasAuthority
    (:Authority
      (if (== (Variables|Default|GetHitComponent) (Variables|Default|GetSM_cp01_02))
        (Utilities|FlowControl|FlipFlop
          (:A
            (CallFunction|OpenDoor))
          (:B
            (CallFunction|CloseDoor)))
        (elif (== (Variables|Default|GetHitComponent) (Variables|Default|GetSM_cp01Button_01))
          (CallFunction|PressMainSwitch)
          (elif (== (Variables|Default|GetHitComponent) (Variables|Default|GetStartSwitch))
            (CallFunction|PressStartButton)
            (elif (== (Variables|Default|GetHitComponent) (Variables|Default|GetResetSwitch))
              (CallFunction|PressResetButton)
              (elif (== (Variables|Default|GetHitComponent) (Variables|Default|GetStopSwitch))
                (CallFunction|PressStopButton)
                (elif (== (Variables|Default|GetHitComponent) (Variables|Default|GetLockSwitch))
                  (Utilities|FlowControl|FlipFlop
                    (:A
                      (CallFunction|RotateLock))
                    (:B
                      (CallFunction|ReverseLock)))
                  (elif (== (Variables|Default|GetHitComponent) (Variables|Default|GetSM_cp01Switch_01))
                    (Utilities|FlowControl|FlipFlop
                      (:A
                        (CallFunction|TurnonFuse01))
                      (:B
                        (CallFunction|TurnOffFuse01)))
                    (elif (== (Variables|Default|GetHitComponent) (Variables|Default|GetSM_cp01Switch_02))
                      (Utilities|FlowControl|FlipFlop
                        (:A
                          (CallFunction|TurnonFuse02))
                        (:B
                          (CallFunction|TurnOffFuse02)))
                      (elif (== (Variables|Default|GetHitComponent) (Variables|Default|GetWireCollision))
                        (if (Variables|Default|GetWire1)
                          (CallFunction|AttachWire))))))))))))))

(fn ConstructionScript
  (bind _returnvalue (Rendering|Material|CreateDynamicMaterialInstance (Variables|Default|GetSK_cp01MWire) 0 (Variables|Default|Getcp%20DM) :!class /Script/Engine.PrimitiveComponent))
  (bind _returnvalue_2 (Rendering|Material|CreateDynamicMaterialInstance (Variables|Default|GetSM_cp01_01) 0 _returnvalue :!class /Script/Engine.PrimitiveComponent))
  (bind _returnvalue_3 (Rendering|Material|CreateDynamicMaterialInstance (Variables|Default|GetSM_cp01_02) 0 _returnvalue_2 :!class /Script/Engine.PrimitiveComponent))
  (bind _returnvalue_4 (Rendering|Material|CreateDynamicMaterialInstance (Variables|Default|GetSM_cp01Button_02) 0 _returnvalue_3 :!class /Script/Engine.PrimitiveComponent))
  (bind _returnvalue_5 (Rendering|Material|CreateDynamicMaterialInstance (Variables|Default|GetSM_cp01Button_03) 0 _returnvalue_4 :!class /Script/Engine.PrimitiveComponent))
  (bind _returnvalue_6 (Rendering|Material|CreateDynamicMaterialInstance (Variables|Default|GetSM_cp01Button_01) 0 _returnvalue_5 :!class /Script/Engine.PrimitiveComponent))
  (bind _returnvalue_7 (Rendering|Material|CreateDynamicMaterialInstance (Variables|Default|GetSM_cp01Button_04) 0 _returnvalue_6 :!class /Script/Engine.PrimitiveComponent))
  (bind _returnvalue_8 (Rendering|Material|CreateDynamicMaterialInstance (Variables|Default|GetSM_cp01Lock_01) 0 _returnvalue_7 :!class /Script/Engine.PrimitiveComponent))
  (bind _returnvalue_9 (Rendering|Material|CreateDynamicMaterialInstance (Variables|Default|GetSM_cp01Switch_01) 0 _returnvalue_8 :!class /Script/Engine.PrimitiveComponent))
  (bind _returnvalue_10 (Rendering|Material|CreateDynamicMaterialInstance (Variables|Default|GetSM_cp01Switch_02) 0 _returnvalue_9 :!class /Script/Engine.PrimitiveComponent))
  (bind _returnvalue_11 (Rendering|Material|CreateDynamicMaterialInstance (Variables|Default|GetSM_cp01WireInside) 0 _returnvalue_10 :!class /Script/Engine.PrimitiveComponent))
  (bind _output_get (Variables|Default|Setcp%20DM _returnvalue_11))
  (Rendering|Material|SetScalarParameterValue _output_get "a:old1" (Variables|Default|GetOld1) :!class /Script/Engine.MaterialInstanceDynamic)
  (Rendering|Material|SetScalarParameterValue (Variables|Default|Getcp%20DM) "b:old2" (Variables|Default|GetOld2) :!class /Script/Engine.MaterialInstanceDynamic)
  (Rendering|Material|SetScalarParameterValue (Variables|Default|Getcp%20DM) "c:full" (Variables|Default|GetFull) :!class /Script/Engine.MaterialInstanceDynamic)
  (Rendering|Material|SetScalarParameterValue (Variables|Default|Getcp%20DM) "d:mainroughness" (Variables|Default|GetMainRoughness) :!class /Script/Engine.MaterialInstanceDynamic)
  (Rendering|Material|SetScalarParameterValue (Variables|Default|Getcp%20DM) "a:lightintensity" (Variables|Default|GetLightIntensity) :!class /Script/Engine.MaterialInstanceDynamic)
  (Rendering|Material|SetScalarParameterValue (Variables|Default|Getcp%20DM) "b:run" (Variables|Default|GetRun) :!class /Script/Engine.MaterialInstanceDynamic)
  (Rendering|Material|SetScalarParameterValue (Variables|Default|Getcp%20DM) "c:open" (Variables|Default|GetClose) :!class /Script/Engine.MaterialInstanceDynamic)
  (Rendering|Material|SetScalarParameterValue (Variables|Default|Getcp%20DM) "d:close" (Variables|Default|GetOpen) :!class /Script/Engine.MaterialInstanceDynamic))