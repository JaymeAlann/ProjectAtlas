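; BP_cp03 is an interactive control panel with a hinged door, start and stop buttons, two parts and a wire.
; ConnectActor routes hit components on authority to toggle the door or buttons, or show components whose flags are set.
; Switch lights the panel blue when on or red when off, only if both parts and wire are visible.
; The construction script chains one dynamic material across the meshes to drive lights and wear.
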(event Custom|ShowPart1
  (Rendering|SetVisibility (Variables|Default|GetSM_cp03Part_01) true false)
  (CallFunction|Switch))

(event Custom|HidePart1
  (Rendering|SetVisibility (Variables|Default|GetSM_cp03Part_01) false false)
  (CallFunction|Switch))

(event Custom|ShowWire
  (Rendering|SetVisibility (Variables|Default|GetSM_cp03Wire_02) true false)
  (CallFunction|Switch))

(event Custom|HIdeWire
  (Rendering|SetVisibility (Variables|Default|GetSM_cp03Wire_02) false false)
  (CallFunction|Switch))

(event Custom|PressStartButton
  (Transformation|SetRelativeLocation (Variables|Default|GetSM_cp03Button_01) "20.709076,16.786776,-20.653952" false false)
  (Transformation|SetRelativeLocation (Variables|Default|GetSM_cp03Button_02) "36.675560,18.786776,-20.653952" false false)
  (Variables|Default|SetSwitchOn? true)
  (CallFunction|Switch))

(event Custom|ReleaseStartButton
  (Transformation|SetRelativeLocation (Variables|Default|GetSM_cp03Button_01) "20.709076,18.786776,-20.653952" false false)
  (CallFunction|Switch))

(event Custom|ShowPart2
  (Rendering|SetVisibility (Variables|Default|GetSM_cp03Part_02) true false)
  (CallFunction|Switch))

(event Custom|HidePart2
  (Rendering|SetVisibility (Variables|Default|GetSM_cp03Part_02) false false)
  (CallFunction|Switch))

(event Custom|CloseDoor
  (Components|Animation|PlayAnimation (Variables|Default|GetSK_cp03MWire) "/Game/ControlPanelPack/Animations/Anim_cp03MWireClose.Anim_cp03MWireClose" false)
  (Components|Timeline|SetPlayRate (Variables|Default|GetSK_cp03MWire) 2.0)
  (bind _doorangle (Timeline|OpenDoorTimeLine Reverse)
    (:Update
      (Transformation|SetRelativeRotation (Variables|Default|GetSM_cp03_02) (Math|Rotator|MakeRotator 0.0 0.0 _doorangle) false false))))

(event Custom|ReleaseStopButton
  (Transformation|SetRelativeLocation (Variables|Default|GetSM_cp03Button_02) "36.675560,18.786776,-20.653952" false false)
  (CallFunction|Switch))

(event Custom|Switch
  (if (Math|Boolean|ANDBoolean (Rendering|IsVisible (Variables|Default|GetSM_cp03Wire_02)) (Rendering|IsVisible (Variables|Default|GetSM_cp03Part_02)) (Rendering|IsVisible (Variables|Default|GetSM_cp03Part_01)))
    (if (Variables|Default|GetSwitchOn?)
      (Rendering|Material|SetScalarParameterValue (Variables|Default|Getcp%20DM) "c:red" 0.0 :!class /Script/Engine.MaterialInstanceDynamic)
      (Rendering|Material|SetScalarParameterValue (Variables|Default|Getcp%20DM) "b:blue" 1.0 :!class /Script/Engine.MaterialInstanceDynamic)
      (else
        (Rendering|Material|SetScalarParameterValue (Variables|Default|Getcp%20DM) "c:red" 1.0 :!class /Script/Engine.MaterialInstanceDynamic)
        (Rendering|Material|SetScalarParameterValue (Variables|Default|Getcp%20DM) "b:blue" 0.0 :!class /Script/Engine.MaterialInstanceDynamic)))
    (else
      (Rendering|Material|SetScalarParameterValue (Variables|Default|Getcp%20DM) "c:red" 0.0 :!class /Script/Engine.MaterialInstanceDynamic)
      (Rendering|Material|SetScalarParameterValue (Variables|Default|Getcp%20DM) "b:blue" 0.0 :!class /Script/Engine.MaterialInstanceDynamic))))

(event Custom|OpenDoor
  (Components|Animation|PlayAnimation (Variables|Default|GetSK_cp03MWire) "/Game/ControlPanelPack/Animations/Anim_cp03MWireOpen.Anim_cp03MWireOpen" false)
  (Components|Animation|SetPosition (Variables|Default|GetSK_cp03MWire) 2.0 true)
  (bind _doorangle (Timeline|OpenDoorTimeLine Play)
    (:Update
      (Transformation|SetRelativeRotation (Variables|Default|GetSM_cp03_02) (Math|Rotator|MakeRotator 0.0 0.0 _doorangle) false false))))

(event Custom|PressStopButton
  (Transformation|SetRelativeLocation (Variables|Default|GetSM_cp03Button_02) "36.675560,16.786776,-20.653952" false false)
  (Transformation|SetRelativeLocation (Variables|Default|GetSM_cp03Button_01) "20.709076,18.786776,-20.653952" false false)
  (Variables|Default|SetSwitchOn? false)
  (CallFunction|Switch))

(event EventConnectActor
  (params (HitComponent :type Actor%20Component%20Object%20Reference))
  (Variables|Default|SetHitComponent HitComponent)
  (Networking|SwitchHasAuthority
    (:Authority
      (if (== (Variables|Default|GetHitComponent) (Variables|Default|GetSM_cp03_02))
        (Utilities|FlowControl|FlipFlop
          (:A
            (CallFunction|OpenDoor))
          (:B
            (CallFunction|CloseDoor)))
        (elif (== (Variables|Default|GetHitComponent) (Variables|Default|GetStartCollision))
          (CallFunction|PressStartButton)
          (elif (== (Variables|Default|GetHitComponent) (Variables|Default|GetStopCollision))
            (CallFunction|PressStopButton)
            (elif (== (Variables|Default|GetHitComponent) (Variables|Default|GetPartCollision))
              (if (Variables|Default|GetPart1)
                (CallFunction|ShowPart1))
              (if (Variables|Default|GetPart2)
                (CallFunction|ShowPart2))
              (elif (== (Variables|Default|GetHitComponent) (Variables|Default|GetWireCollision))
                (if (Variables|Default|GetWire)
                  (CallFunction|ShowWire))))))))))

(event EventBeginPlay
  (Components|Animation|PlayAnimation (Variables|Default|GetSK_cp03MWire) "/Game/ControlPanelPack/Animations/Anim_cp03MWireClose.Anim_cp03MWireClose" false)
  (Components|Timeline|SetPlayRate (Variables|Default|GetSK_cp03MWire) 2.0)
  (CallFunction|Switch)
  (Utilities|FlowControl|Sequence
    (:then_0
      (if (Variables|Default|GetPart1)
        _
        (else
          (CallFunction|HidePart1)))
      (CallFunction|Switch))
    (:then_1
      (if (Variables|Default|GetPart2)
        _
        (else
          (CallFunction|HidePart2)))
      (CallFunction|Switch))
    (:then_2
      (if (Variables|Default|GetWire)
        _
        (else
          (CallFunction|HIdeWire)))
      (CallFunction|Switch))))

(fn ConstructionScript
  (bind _returnvalue (Rendering|Material|CreateDynamicMaterialInstance (Variables|Default|GetSM_cp03_01) 0 (Variables|Default|Getcp%20DM) :!class /Script/Engine.PrimitiveComponent))
  (bind _returnvalue_2 (Rendering|Material|CreateDynamicMaterialInstance (Variables|Default|GetSK_cp03MWire) 0 _returnvalue :!class /Script/Engine.PrimitiveComponent))
  (bind _returnvalue_3 (Rendering|Material|CreateDynamicMaterialInstance (Variables|Default|GetSM_cp03Wire_02) 0 _returnvalue_2 :!class /Script/Engine.PrimitiveComponent))
  (bind _returnvalue_4 (Rendering|Material|CreateDynamicMaterialInstance (Variables|Default|GetSM_cp03Part_01) 0 _returnvalue_3 :!class /Script/Engine.PrimitiveComponent))
  (bind _returnvalue_5 (Rendering|Material|CreateDynamicMaterialInstance (Variables|Default|GetSM_cp03Part_02) 0 _returnvalue_4 :!class /Script/Engine.PrimitiveComponent))
  (bind _returnvalue_6 (Rendering|Material|CreateDynamicMaterialInstance (Variables|Default|GetSM_cp03_02) 0 _returnvalue_5 :!class /Script/Engine.PrimitiveComponent))
  (bind _returnvalue_7 (Rendering|Material|CreateDynamicMaterialInstance (Variables|Default|GetSM_cp03Button_02) 0 _returnvalue_6 :!class /Script/Engine.PrimitiveComponent))
  (bind _returnvalue_8 (Rendering|Material|CreateDynamicMaterialInstance (Variables|Default|GetSM_cp03Button_01) 0 _returnvalue_7 :!class /Script/Engine.PrimitiveComponent))
  (bind _output_get (Variables|Default|Setcp%20DM _returnvalue_8))
  (Rendering|Material|SetScalarParameterValue _output_get "a:old1" (Variables|Default|GetOld1) :!class /Script/Engine.MaterialInstanceDynamic)
  (Rendering|Material|SetScalarParameterValue (Variables|Default|Getcp%20DM) "b:old2" (Variables|Default|GetOld2) :!class /Script/Engine.MaterialInstanceDynamic)
  (Rendering|Material|SetScalarParameterValue (Variables|Default|Getcp%20DM) "c:full" (Variables|Default|GetFull) :!class /Script/Engine.MaterialInstanceDynamic)
  (Rendering|Material|SetScalarParameterValue (Variables|Default|Getcp%20DM) "d:mainroughness" (Variables|Default|GetMainRoughness) :!class /Script/Engine.MaterialInstanceDynamic)
  (Rendering|Material|SetScalarParameterValue (Variables|Default|Getcp%20DM) "a:lightintensity" (Variables|Default|GetLightIntensity) :!class /Script/Engine.MaterialInstanceDynamic)
  (Rendering|Material|SetScalarParameterValue (Variables|Default|Getcp%20DM) "b:blue" (Variables|Default|GetBlue) :!class /Script/Engine.MaterialInstanceDynamic)
  (Rendering|Material|SetScalarParameterValue (Variables|Default|Getcp%20DM) "c:red" (Variables|Default|GetRed) :!class /Script/Engine.MaterialInstanceDynamic))