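; Interactive control panel actor with a hinged door, two wires, fuse, main button and two side switches driving indicator lights.
; ConnectActor, on authority, maps the hit component to door, wire or FlipFlop toggle actions; both wire reveals check Wire1.
; Switch re-evaluates the state: with wires and fuse in place, the buttons select auto, motor or overload.
; The construction script chains one dynamic material through all meshes, so parameter changes affect the whole panel.
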(event Custom|PressFuse
  (Transformation|SetRelativeRotation (Variables|Default|GetSM_cp04Switch_01) "0.000000, 0,-30.000000" false false)
  (Variables|Default|SetFuseOn? true)
  (CallFunction|Switch))

(event Custom|ShowWire1
  (Rendering|SetVisibility (Variables|Default|GetSM_cp04Wire_01) true false)
  (CallFunction|Switch))

(event Custom|HideWire1
  (Rendering|SetVisibility (Variables|Default|GetSM_cp04Wire_01) false false)
  (CallFunction|Switch))

(event Custom|PressMainButton
  (Transformation|SetRelativeLocation (Variables|Default|GetSM_cp04Switch_04) "42.758091,0.220947,53.812836" false false)
  (Variables|Default|SetMainButtonOn? true)
  (CallFunction|Switch))

(event Custom|ReleaseMainButton
  (Transformation|SetRelativeLocation (Variables|Default|GetSM_cp04Switch_04) "45.758091,0.220947,53.812836" false false)
  (Variables|Default|SetMainButtonOn? false)
  (CallFunction|Switch))

(event Custom|CloseDoor
  (bind _doorangle (Timeline|OpenDoorTimeLine Reverse)
    (:Update
      (Transformation|SetRelativeRotation (Variables|Default|GetSM_cp04_02) (Math|Rotator|MakeRotator 0.0 0.0 _doorangle) false false))))

(event Custom|OpenDoor
  (bind _doorangle (Timeline|OpenDoorTimeLine Play)
    (:Update
      (Transformation|SetRelativeRotation (Variables|Default|GetSM_cp04_02) (Math|Rotator|MakeRotator 0.0 0.0 _doorangle) false false))))

(event Custom|PressSwitch02
  (Transformation|SetRelativeRotation (Variables|Default|GetSM_cp04Switch_03) "30.000000, 0, 0" false false)
  (Variables|Default|SetSide02ButtonOn? true)
  (CallFunction|Switch))

(event Custom|ReleaseSwitch02
  (Transformation|SetRelativeRotation (Variables|Default|GetSM_cp04Switch_03) "-30.000000, 0, 0" false false)
  (Variables|Default|SetSide02ButtonOn? false)
  (CallFunction|Switch))

(event Custom|PressSwitch01
  (Transformation|SetRelativeRotation (Variables|Default|GetSM_cp04Switch_02) "30.000000, 0, 0" false false)
  (Variables|Default|SetSide01ButtonOn? true)
  (CallFunction|Switch))

(event Custom|ReleaseSwitch01
  (Transformation|SetRelativeRotation (Variables|Default|GetSM_cp04Switch_02) "-30.000000, 0, 0" false false)
  (Variables|Default|SetSide01ButtonOn? false)
  (CallFunction|Switch))

(event Custom|HideWire2
  (Rendering|SetVisibility (Variables|Default|GetSM_cp04Wire_02) false false)
  (CallFunction|Switch))

(event Custom|ShowWire2
  (Rendering|SetVisibility (Variables|Default|GetSM_cp04Wire_02) true false)
  (CallFunction|Switch))

(event Custom|Switch
  (if (Math|Boolean|ANDBoolean (Rendering|IsVisible (Variables|Default|GetSM_cp04Wire_01)) (Rendering|IsVisible (Variables|Default|GetSM_cp04Wire_02)) (Variables|Default|GetFuseOn?))
    (if (Variables|Default|GetMainButtonOn?)
      (if (and (Variables|Default|GetSide01ButtonOn?) (Variables|Default|GetSide02ButtonOn?))
        (Rendering|Material|SetScalarParameterValue (Variables|Default|Getcp%20DM) "b:auto" 1.0 :!class /Script/Engine.MaterialInstanceDynamic)
        (Rendering|Material|SetScalarParameterValue (Variables|Default|Getcp%20DM) "c:motor" 0.0 :!class /Script/Engine.MaterialInstanceDynamic)
        (Rendering|Material|SetScalarParameterValue (Variables|Default|Getcp%20DM) "d:overload" 0.0 :!class /Script/Engine.MaterialInstanceDynamic)
        (else
          (Rendering|Material|SetScalarParameterValue (Variables|Default|Getcp%20DM) "b:auto" 0.0 :!class /Script/Engine.MaterialInstanceDynamic)
          (Rendering|Material|SetScalarParameterValue (Variables|Default|Getcp%20DM) "c:motor" 1.0 :!class /Script/Engine.MaterialInstanceDynamic)
          (Rendering|Material|SetScalarParameterValue (Variables|Default|Getcp%20DM) "d:overload" 0.0 :!class /Script/Engine.MaterialInstanceDynamic)))
      (else
        (Rendering|Material|SetScalarParameterValue (Variables|Default|Getcp%20DM) "b:auto" 0.0 :!class /Script/Engine.MaterialInstanceDynamic)
        (Rendering|Material|SetScalarParameterValue (Variables|Default|Getcp%20DM) "c:motor" 0.0 :!class /Script/Engine.MaterialInstanceDynamic)
        (Rendering|Material|SetScalarParameterValue (Variables|Default|Getcp%20DM) "d:overload" 1.0 :!class /Script/Engine.MaterialInstanceDynamic)))
    (else
      (Rendering|Material|SetScalarParameterValue (Variables|Default|Getcp%20DM) "b:auto" 0.0 :!class /Script/Engine.MaterialInstanceDynamic)
      (Rendering|Material|SetScalarParameterValue (Variables|Default|Getcp%20DM) "c:motor" 0.0 :!class /Script/Engine.MaterialInstanceDynamic)
      (Rendering|Material|SetScalarParameterValue (Variables|Default|Getcp%20DM) "d:overload" 0.0 :!class /Script/Engine.MaterialInstanceDynamic))))

(event Custom|ReleaseFuse
  (Transformation|SetRelativeRotation (Variables|Default|GetSM_cp04Switch_01) "0.000000, 0,30.000000" false false)
  (Variables|Default|SetFuseOn? false)
  (CallFunction|Switch))

(event EventConnectActor
  (params (HitComponent :type Actor%20Component%20Object%20Reference))
  (Variables|Default|SetHitComponent HitComponent)
  (Networking|SwitchHasAuthority
    (:Authority
      (if (== (Variables|Default|GetHitComponent) (Variables|Default|GetSM_cp04_02))
        (Utilities|FlowControl|FlipFlop
          (:A
            (CallFunction|OpenDoor))
          (:B
            (CallFunction|CloseDoor)))
        (elif (== (Variables|Default|GetHitComponent) (Variables|Default|GetWireCollision))
          (if (Variables|Default|GetWire1)
            (CallFunction|ShowWire1))
          (if (Variables|Default|GetWire1)
            (CallFunction|ShowWire2))
          (elif (== (Variables|Default|GetHitComponent) (Variables|Default|GetSwitch03Collision))
            (Utilities|FlowControl|FlipFlop
              (:A
                (CallFunction|PressMainButton))
              (:B
                (CallFunction|ReleaseMainButton)))
            (elif (== (Variables|Default|GetHitComponent) (Variables|Default|GetSwitch02Collision))
              (Utilities|FlowControl|FlipFlop
                (:A
                  (CallFunction|PressSwitch02))
                (:B
                  (CallFunction|ReleaseSwitch02)))
              (elif (== (Variables|Default|GetHitComponent) (Variables|Default|GetSwitch01Collision))
                (Utilities|FlowControl|FlipFlop
                  (:A
                    (CallFunction|PressSwitch01))
                  (:B
                    (CallFunction|ReleaseSwitch01)))
                (elif (== (Variables|Default|GetHitComponent) (Variables|Default|GetSM_cp04Switch_01))
                  (Utilities|FlowControl|FlipFlop
                    (:A
                      (CallFunction|PressFuse))
                    (:B
                      (CallFunction|ReleaseFuse))))))))))))

(event EventBeginPlay
  (CallFunction|Switch)
  (Utilities|FlowControl|Sequence
    (:then_0
      (if (Variables|Default|GetWire1)
        _
        (else
          (CallFunction|HideWire1)))
      (CallFunction|Switch))
    (:then_1
      (if (Variables|Default|GetWire2)
        _
        (else
          (CallFunction|HideWire2)))
      (CallFunction|Switch))))

(fn ConstructionScript
  (bind _returnvalue (Rendering|Material|CreateDynamicMaterialInstance (Variables|Default|GetSM_cp04_01) 0 (Variables|Default|Getcp%20DM) :!class /Script/Engine.PrimitiveComponent))
  (bind _returnvalue_2 (Rendering|Material|CreateDynamicMaterialInstance (Variables|Default|GetSM_cp04Switch_01) 0 _returnvalue :!class /Script/Engine.PrimitiveComponent))
  (bind _returnvalue_3 (Rendering|Material|CreateDynamicMaterialInstance (Variables|Default|GetSM_cp04Switch_02) 0 _returnvalue_2 :!class /Script/Engine.PrimitiveComponent))
  (bind _returnvalue_4 (Rendering|Material|CreateDynamicMaterialInstance (Variables|Default|GetSM_cp04Switch_03) 0 _returnvalue_3 :!class /Script/Engine.PrimitiveComponent))
  (bind _returnvalue_5 (Rendering|Material|CreateDynamicMaterialInstance (Variables|Default|GetSM_cp04Switch_04) 0 _returnvalue_4 :!class /Script/Engine.PrimitiveComponent))
  (bind _returnvalue_6 (Rendering|Material|CreateDynamicMaterialInstance (Variables|Default|GetSM_cp04Wire_01) 0 _returnvalue_5 :!class /Script/Engine.PrimitiveComponent))
  (bind _returnvalue_7 (Rendering|Material|CreateDynamicMaterialInstance (Variables|Default|GetSM_cp04Wire_02) 0 _returnvalue_6 :!class /Script/Engine.PrimitiveComponent))
  (bind _returnvalue_8 (Rendering|Material|CreateDynamicMaterialInstance (Variables|Default|GetSM_cp04_02) 0 _returnvalue_7 :!class /Script/Engine.PrimitiveComponent))
  (bind _output_get (Variables|Default|Setcp%20DM _returnvalue_8))
  (Rendering|Material|SetScalarParameterValue _output_get "a:old1" (Variables|Default|GetOld1) :!class /Script/Engine.MaterialInstanceDynamic)
  (Rendering|Material|SetScalarParameterValue (Variables|Default|Getcp%20DM) "b:old2" (Variables|Default|GetOld2) :!class /Script/Engine.MaterialInstanceDynamic)
  (Rendering|Material|SetScalarParameterValue (Variables|Default|Getcp%20DM) "c:full" (Variables|Default|GetFull) :!class /Script/Engine.MaterialInstanceDynamic)
  (Rendering|Material|SetScalarParameterValue (Variables|Default|Getcp%20DM) "d:mainroughness" (Variables|Default|GetMainRoughness) :!class /Script/Engine.MaterialInstanceDynamic)
  (Rendering|Material|SetScalarParameterValue (Variables|Default|Getcp%20DM) "a:lightintensity" (Variables|Default|GetLightIntensity) :!class /Script/Engine.MaterialInstanceDynamic)
  (Rendering|Material|SetScalarParameterValue (Variables|Default|Getcp%20DM) "b:auto" (Variables|Default|GetAuto) :!class /Script/Engine.MaterialInstanceDynamic)
  (Rendering|Material|SetScalarParameterValue (Variables|Default|Getcp%20DM) "c:motor" (Variables|Default|GetMotor) :!class /Script/Engine.MaterialInstanceDynamic)
  (Rendering|Material|SetScalarParameterValue (Variables|Default|Getcp%20DM) "d:overload" (Variables|Default|GetOverload) :!class /Script/Engine.MaterialInstanceDynamic)
  (Rendering|Material|SetScalarParameterValue (Variables|Default|Getcp%20DM) "e:light" (Variables|Default|GetLight) :!class /Script/Engine.MaterialInstanceDynamic))